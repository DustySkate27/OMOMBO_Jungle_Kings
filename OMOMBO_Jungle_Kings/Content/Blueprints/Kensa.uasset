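; Kensa is an enemy that smoothly turns toward Pedro within its vision field and repeatedly spawns DevilsBombs while he is in shooting range.
; Tick-driven counters, used instead of Delays, run the shot cooldown, post-hit invincibility and temporary health-widget display.
; Myasai-tagged hitbox overlaps damage it; on death it destroys itself and increments Pedro's EnemyCount, which triggers his ActivateDoor at a set count.
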(event `self.ReceiveBeginPlay`
  ; Start
  (`self.LifeInitializer`)
  (bind _returnvalue (`GameplayStatics.GetActorOfClass` "/Game/ThirdPerson/Blueprints/Myasai.Myasai_C"))
  (set `self.Myasai` _returnvalue)
  (bind _aswb_kensa_hp (cast `/Game/ThirdPerson/Blueprints/WB_KensaHP` (`WidgetComponent.GetWidget` (`self.KensaHP`))))
  (set `self.As WB Kensa HP` _aswb_kensa_hp))

(event `self.ReceiveTick`
  (params (DeltaSeconds :type "Float (single-precision)"))
  ; Update
  (if (`self.ShowHP`)
    (`self.HPLeft`))
  (`self.LookAtPedro`)
  (`self.IFrames`)
  (`self.ShootCooldown`) ; Esta función debería poder subplantar delay\nOnRange == True\nEsta función pone en True ableToShoot
)

(event `self.ShootRange.OnComponentBeginOverlap`
  (params (OverlappedComponent :type "PrimitiveComponent Object Reference") (OtherActor :type "Actor Object Reference") (OtherComp :type "PrimitiveComponent Object Reference") (OtherBodyIndex :type Integer) (bFromSweep :type Boolean) (SweepResult :type "HitResult Structure (by ref)"))
  ; Trank paaa, ya no hay mas delay, solo contadores OOOAAA
  (if (`self.ActorHasTag` OtherActor "Pedro")
    (set `self.onRange` true)))

(event `Shoot`
  ; Trank paaa, ya no hay mas delay, solo contadores OOOAAA
  (bind _returnvalue (`|SpawnActorFromClass` "/Game/ThirdPerson/Blueprints/DevilsBomb.DevilsBomb_C" (`SceneComponent.K2_GetComponentToWorld` (`self.DevilsBombSpawn`)) "AlwaysSpawn" "MultiplyWithRoot" null null))
  (set `self.DevilsBomb` _returnvalue))

(event `self.ShootRange.OnComponentEndOverlap`
  (params (OverlappedComponent :type "PrimitiveComponent Object Reference") (OtherActor :type "Actor Object Reference") (OtherComp :type "PrimitiveComponent Object Reference") (OtherBodyIndex :type Integer))
  ; Trank paaa, ya no hay mas delay, solo contadores OOOAAA
  (if (`self.ActorHasTag` OtherActor "Pedro")
    (set `self.ableToShoot` false)
    (set `self.onRange` false)))

(event `self.VisionField.OnComponentBeginOverlap`
  (params (OverlappedComponent :type "PrimitiveComponent Object Reference") (OtherActor :type "Actor Object Reference") (OtherComp :type "PrimitiveComponent Object Reference") (OtherBodyIndex :type Integer) (bFromSweep :type Boolean) (SweepResult :type "HitResult Structure (by ref)"))
  ; Obtención de campo de vision
  (bind _aspedro (cast `/Game/ThirdPerson/Blueprints/Pedro` OtherActor))
  (set `self.Pedro` _aspedro)
  (set `self.onVision` true))

(event `self.KensaHitbox.OnComponentBeginOverlap`
  (params (OverlappedComponent :type "PrimitiveComponent Object Reference") (OtherActor :type "Actor Object Reference") (OtherComp :type "PrimitiveComponent Object Reference") (OtherBodyIndex :type Integer) (bFromSweep :type Boolean) (SweepResult :type "HitResult Structure (by ref)"))
  ; Hit & Kill count
  (if (`self.ActorHasTag` OtherActor "Myasai")
    (`self.DamageByInt` 25)
    (bind _dead (`self.isAlive`))
    (if _dead
      (bind _result (`/Engine/EditorBlueprintResources/StandardMacros.IncrementInt` (`/Game/ThirdPerson/Blueprints/Pedro.EnemyCount` (`self.Pedro`)))
        (:`  `
          (if (== _result 3)
            (`/Game/ThirdPerson/Blueprints/Pedro.Activate Door` (`self.Pedro`))))))))

(event `self.VisionField.OnComponentEndOverlap`
  (params (OverlappedComponent :type "PrimitiveComponent Object Reference") (OtherActor :type "Actor Object Reference") (OtherComp :type "PrimitiveComponent Object Reference") (OtherBodyIndex :type Integer))
  ; Obtención de campo de vision
  (if (`self.ActorHasTag` OtherActor "Pedro")
    (set `self.onVision` false)))

(fn `DamageByInt`
  (params (Damage :type Integer))
  (bind (_reductedlife _activateiframes) (`/Game/Libraries/BasicFunctions.TakeDamage` (`self.Life`) Damage (`self.gotHit`)))
  (set `self.Life` _reductedlife)
  (set `self.gotHit` _activateiframes)
  (set `self.ShowHP` true)
  (set `self.lifeTextCounter` 0.0)
  (set `self.InvincibilityFrames` 0.0))

(fn `HPLeft`
  (bind _output_get (set `self.lifeTextCounter` (+ (`self.lifeTextCounter`) (`GameplayStatics.GetWorldDeltaSeconds`))))
  (if (<= _output_get 3.0)
    (`SceneComponent.SetVisibility` (`self.KensaHP`) true true)
    (`/Game/ThirdPerson/Blueprints/WB_KensaHP.ChangeHealthText` (`self.As WB Kensa HP`) (`self.Life`))
    (else
      (`SceneComponent.SetVisibility` (`self.KensaHP`) false true)
      (set `self.ShowHP` false))))

(fn `IFrames`
  ; Si fue golpeado, empieza un contador. Cuando se superan los 0.5s, se pone en false "gotHit"
  (bind (_keepiframesactive _currenticounter) (`/Game/Libraries/BasicFunctions.CheckInvincible` (`self.gotHit`) (`self.InvincibilityFrames`) 5.0 self))
  (set `self.gotHit` _keepiframesactive)
  (set `self.InvincibilityFrames` _currenticounter))

(fn `isAlive`
  (returns (Dead :type Boolean))
  (if (<= (`self.life`) 0)
    (`self.K2_DestroyActor`)
    (return true)))

(fn `LifeInitializer`
  (set `self.life` 100))

(fn `LookAtPedro`
  (bind (_returnvalue_roll _returnvalue_pitch _returnvalue_yaw) (`KismetMathLibrary.BreakRotator` (`KismetMathLibrary.FindLookAtRotation` (`self.K2_GetActorLocation`) (`self.K2_GetActorLocation` (`self.Pedro`)))))
  (if (`self.onVision`)
    (if (`KismetSystemLibrary.IsValid` (`self.Pedro`))
      (`self.K2_SetActorRotation` (`KismetMathLibrary.RInterpTo` (`self.K2_GetActorRotation`) (`KismetMathLibrary.MakeRotator` 0.0 0.0 _returnvalue_yaw) (`GameplayStatics.GetWorldDeltaSeconds`) 10.0)))))

(fn `ShootCooldown`
  ; Mientras "OnRange" sea true, corre el contador. Cuando "AbleToShoot" es true, se dispara.
  ; Si "OnRange" es false, mantiene en 0 el contador.
  (if (`self.onRange`)
    (bind _output_get (set `self.devilsBombCooldown` (+ (`self.devilsBombCooldown`) (`GameplayStatics.GetWorldDeltaSeconds`))))
    (set `self.ableToShoot` (> _output_get 1.5))
    (if (`self.ableToShoot`)
      (`self.Shoot`)
      (set `self.devilsBombCooldown` 0.0 :!label _label))
    (else
      (goto _label))))

(fn `UserConstructionScript`)