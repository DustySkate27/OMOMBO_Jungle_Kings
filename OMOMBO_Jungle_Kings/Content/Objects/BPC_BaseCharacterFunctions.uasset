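; Actor component of shared character functions that apply integer damage to health variables passed in by reference.
; Each function skips if GotHit is already set, otherwise subtracts damage, resets the IFrames timer and sets GotHit, leaving invincibility timing to the caller.
; The widget-included variant also flags the HP widget to show and resets its counter.
; The event graph is empty.
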(fn `DamageByInt`
  (params (CurrentHealth :type "Integer (by ref)") (Damage :type Integer) (GotHit :type "Boolean (by ref)") (IFrames :type "Float (double-precision) (by ref)"))
  (if (not (`local.GotHit`))
    (`|VariableSetRef` (`local.CurrentHealth`) (- CurrentHealth Damage))
    (`|VariableSetRef` (`local.IFrames`))
    (`|VariableSetRef` (`local.GotHit`) true)))

(fn `DamageByInt(WidgetIncluded)`
  (params (CurrentHealth :type "Integer (by ref)") (Damage :type Integer) (GotHit :type "Boolean (by ref)") (IFrames :type "Float (double-precision) (by ref)") (ShowHPWid :type Boolean) (HPWidCounter :type "Float (double-precision)"))
  (if (not (`local.gotHit`))
    (`|VariableSetRef` (`local.CurrentHealth`) (- CurrentHealth Damage))
    (`|VariableSetRef` (`local.IFrames`))
    (`|VariableSetRef` (`local.ShowHPWid`) true)
    (`|VariableSetRef` (`local.HPWidCounter`))
    (`|VariableSetRef` (`local.GotHit`) true)))