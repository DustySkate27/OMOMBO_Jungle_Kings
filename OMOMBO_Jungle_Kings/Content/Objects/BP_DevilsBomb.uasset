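; BP_DevilsBomb is a projectile bomb that poisons Pedro when its hitbox overlaps him.
; It caches the BP_Pedro actor on BeginPlay and sets that actor's Poisoned flag when BombHitbox overlaps an actor tagged Pedro.
; The construction script sets the ProjectileMovement initial speed from the Velocity variable, falling back to a default when it is zero.
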(event `self.ReceiveBeginPlay`
  (bind _returnvalue (`GameplayStatics.GetActorOfClass` "/Game/Objects/BP_Pedro.BP_Pedro_C"))
  (set `self.Pedro` _returnvalue))

(event `self.BombHitbox.OnComponentBeginOverlap`
  (params (OverlappedComponent :type "PrimitiveComponent Object Reference") (OtherActor :type "Actor Object Reference") (OtherComp :type "PrimitiveComponent Object Reference") (OtherBodyIndex :type Integer) (bFromSweep :type Boolean) (SweepResult :type "HitResult Structure (by ref)"))
  (if (`self.ActorHasTag` OtherActor "Pedro")
    (set `/Game/Objects/BP_Pedro.poisoned` true (`self.Pedro`))))

(fn `UserConstructionScript`
  (bind _projectilemovement (`self.ProjectileMovement`))
  (if (== (`self.velocity`) 0.0)
    (set `ProjectileMovementComponent.InitialSpeed` 1000.0 _projectilemovement)
    (else
      (set `ProjectileMovementComponent.InitialSpeed` (`self.velocity`) _projectilemovement))))