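; BP_Myasai is an object bound to Pedro that trails the character and can be launched to a strike point.
; BeginPlay caches Pedro's follow and strike points, then Tick polls Pedro's activation and launch flags.
; While activated, it interpolates to the follow point with collision disabled, matching Pedro's rotation.
; On launch, it interpolates faster toward the strike point, clearing the flag and enabling blocking collision once close.
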(event `self.ReceiveBeginPlay`
  ; Start
  (bind _returnvalue (`GameplayStatics.GetActorOfClass` "/Game/Objects/BP_Pedro.BP_Pedro_C"))
  (bind _output_get (set `self.Pedro` _returnvalue))
  (set `self.FollowPoint` (`/Game/Objects/BP_Pedro.MyasaiFollowPoint` _output_get))
  (set `self.StrikePoint` (`/Game/Objects/BP_Pedro.MyasaiStrike` _output_get)))

(event `self.ReceiveTick`
  (params (DeltaSeconds :type "Float (single-precision)"))
  ; Update
  (`self.IveBeenInvoked`)
  (`self.ImAttacking`))

(fn `ImAttacking`
  (if (and (`KismetSystemLibrary.IsValid` (`self.StrikePoint`)) (`/Game/Objects/BP_Pedro.myasaiLaunch` (`self.Pedro`)))
    (`self.K2_SetActorLocationAndRotation` (`KismetMathLibrary.VInterpTo` (`self.K2_GetActorLocation`) (`SceneComponent.K2_GetComponentLocation` (`self.StrikePoint`)) (`GameplayStatics.GetWorldDeltaSeconds`) 40.0) (`self.K2_GetActorRotation` (`self.Pedro`)))
    (if (== (`self.K2_GetActorLocation`) (`SceneComponent.K2_GetComponentLocation` (`self.StrikePoint`)) :`ErrorTolerance` 20.0)
      (set `/Game/Objects/BP_Pedro.myasaiLaunch` false (`self.Pedro`))
      (`PrimitiveComponent.SetCollisionProfileName` (`self.MyasaiHitbox`) "BlockAll" true))))

(fn `IveBeenInvoked`
  (if (and (`/Game/Objects/BP_Pedro.myasaiActivation` (`self.Pedro`)) (`KismetSystemLibrary.IsValid` (`self.FollowPoint`)))
    (`PrimitiveComponent.SetCollisionProfileName` (`self.MyasaiHitbox`) "NoCollision" true)
    (`self.K2_SetActorLocationAndRotation` (`KismetMathLibrary.VInterpTo` (`self.K2_GetActorLocation`) (`SceneComponent.K2_GetComponentLocation` (`self.FollowPoint`)) (`GameplayStatics.GetWorldDeltaSeconds`) 20.0) (`self.K2_GetActorRotation` (`self.Pedro`)))))

(fn `IveBeenThrown`)

(fn `UserConstructionScript`)